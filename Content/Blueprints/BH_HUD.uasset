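; HUD Blueprint that draws the player's attempt value and score on screen, then a mission-complete summary once the game is won.
; DrawHUD checks GameWon each frame and calls either DrawInGame or DrawEndGame.
; Both draw canvas text with DrawText, using viewport and text size to position it: along the top during play, centred in red at the end.
; The end screen labels PlayerAttempt as seconds.
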(event `self.ReceiveDrawHUD`
  (params (SizeX :type Integer) (SizeY :type Integer))
  (if (`self.GameWon`)
    (`self.DrawEndGame`)
    (else
      (`self.DrawInGame`))))

(fn `DrawEndGame`
  (bind _screenfont (`self.ScreenFont`))
  (bind _screenfont_2 (`self.ScreenFont`))
  (bind (_x _y) (`KismetMathLibrary.BreakVector2D` (`WidgetLayoutLibrary.GetViewportSize`)))
  (bind (_x_2 _y_2) (`KismetMathLibrary.BreakVector2D` (`WidgetLayoutLibrary.GetViewportSize`)))
  (bind _returnvalue (`KismetStringLibrary.Concat_StrStr` "Mission Complete!" (`KismetStringLibrary.Conv_DoubleToString` (`self.PlayerAttempt`)) "seconds!"))
  (bind _returnvalue_2 (`KismetStringLibrary.Concat_StrStr` "With " (`KismetStringLibrary.Conv_IntToString` (`self.point`)) " points!"))
  (bind (_outwidth _outheight) (`self.GetTextSize` _returnvalue _screenfont_2 2.0))
  (bind (_outwidth_2 _outheight_2) (`self.GetTextSize` _returnvalue_2 _screenfont 2.0))
  (`self.DrawText` _returnvalue (struct :`R` 1.0 :`A` 1.0) (- (* _x_2 0.5) (* _outwidth 0.5)) (- (* _y_2 0.5) (* _outheight 0.5)) _screenfont_2 2.0)
  (`self.DrawText` _returnvalue_2 (struct :`R` 1.0 :`A` 1.0) (- (* _x 0.5) (* _outwidth_2 0.5)) (- (* _y 0.5) (* _outheight_2 -1.2)) _screenfont 2.0))

(fn `DrawInGame`
  (bind _screenfont (`self.ScreenFont`))
  (bind _screenfont_2 (`self.ScreenFont`))
  (bind _returnvalue (`KismetStringLibrary.Conv_DoubleToString` (`self.PlayerAttempt`)))
  (bind _returnvalue_2 (`KismetStringLibrary.Concat_StrStr` (`KismetStringLibrary.Conv_IntToString` (`self.point`)) "points!"))
  (`self.DrawText` _returnvalue (struct :`R` 1.0 :`G` 1.0 :`B` 1.0 :`A` 1.0) (- (* (`KismetMathLibrary.BreakVector2D` (`WidgetLayoutLibrary.GetViewportSize`)) 0.5) (* (`self.GetTextSize` _returnvalue _screenfont_2 2.0) 0.5)) 0.0 _screenfont_2 2.0)
  (`self.DrawText` _returnvalue_2 (struct :`R` 1.0 :`G` 1.0 :`B` 1.0 :`A` 1.0) (- (* (`KismetMathLibrary.BreakVector2D` (`WidgetLayoutLibrary.GetViewportSize`)) 0.8) (* (`self.GetTextSize` _returnvalue_2 _screenfont 2.0) 0.5)) 0.0 _screenfont 2.0))

(fn `UserConstructionScript`)