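; Enemy actor that moves along a timeline-driven path and kills the player character through a box collision.
; BeginPlay caches the mesh's world location; Tick hides the text render and plays the Move timeline, which offsets the mesh along world Y from that start.
; When a BH_Character ends overlap with the box, rather than begins it, player 0's character is destroyed and a death sound plays at world origin.
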(event `self.ReceiveTick`
  (params (DeltaSeconds :type "Float (single-precision)"))
  (`SceneComponent.SetVisibility` (`self.TextRender`) false false)
  (bind (_direction `_새_트랙_0`) (`Timeline|move`)
    (:`Update`
      (`SceneComponent.K2_SetWorldLocation` (`self.StaticMeshComponent`) (+ (`self.StartLocation`) (`KismetMathLibrary.MakeVector` 0.0 (.y `_새_트랙_0`))) false false))))

(event `self.ReceiveBeginPlay`
  (set `self.StartLocation` (`SceneComponent.K2_GetComponentLocation` (`self.StaticMeshComponent`))))

(event `self.BoxCollision.OnComponentEndOverlap`
  (params (OverlappedComponent :type "PrimitiveComponent Object Reference") (OtherActor :type "Actor Object Reference") (OtherComp :type "PrimitiveComponent Object Reference") (OtherBodyIndex :type Integer))
  (if (== (`GameplayStatics.GetObjectClass` OtherActor) "/Game/BarrelHopper/Character/BH_Character.BH_Character_C")
    (`self.K2_DestroyActor` (`GameplayStatics.GetPlayerCharacter` 0))
    (`GameplayStatics.PlaySoundAtLocation` "/Game/BarrelHopper/sound/DeathSound.DeathSound" (0.0 0.0 0.0) (struct) 1.0 1.0 0.0 null null null)))

(fn `Interact`
  (returns (Success :type Boolean)))

(fn `UserConstructionScript`)