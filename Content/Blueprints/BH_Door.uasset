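; BH_Door is an interactable door that slides along the vertical axis to open.
; Entering its box collision as a BH_Character reveals a text render, with no end-overlap logic to hide it.
; Interact calls OpenDoor and returns false; OpenDoor hides the text and plays a timeline that offsets the mesh in Z from its location cached at BeginPlay.
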(event `self.ReceiveBeginPlay`
  (set `self.StartLocation` (`SceneComponent.K2_GetComponentLocation` (`self.StaticMeshComponent`))))

(event `OpenDoor`
  (`SceneComponent.SetVisibility` (`self.TextRender`) false false)
  (bind (_direction `_새_트랙_0`) (`Timeline|DoorOpeningTimeLine`)
    (:`Update`
      (`SceneComponent.K2_SetWorldLocation` (`self.StaticMeshComponent`) (+ (`self.StartLocation`) (`KismetMathLibrary.MakeVector` 0.0 0.0 `_새_트랙_0`)) false false))))

(event `self.BoxCollision.OnComponentBeginOverlap`
  (params (OverlappedComponent :type "PrimitiveComponent Object Reference") (OtherActor :type "Actor Object Reference") (OtherComp :type "PrimitiveComponent Object Reference") (OtherBodyIndex :type Integer) (bFromSweep :type Boolean) (SweepResult :type "HitResult Structure (by ref)"))
  (if (== (`GameplayStatics.GetObjectClass` OtherActor) "/Game/BarrelHopper/Character/BH_Character.BH_Character_C")
    (`SceneComponent.SetVisibility` (`self.TextRender`) true false)))

(fn `Interact`
  (returns (Success :type Boolean))
  (`self.OpenDoor`)
  (return false))

(fn `UserConstructionScript`)