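; NPC1 is a talkable NPC that shows floating text and disappears when the player re-enters its trigger after talking.
; A BH_Character entering the Box shows TextRender, and leaving hides it.
; Talk fires the what'sup event, which reveals TextRender1 and plays a male laugh cue at the world origin, then returns false.
; TextRender1's visibility doubles as the talked-to flag: if visible on overlap, the actor destroys itself.
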(event `self.ReceiveBeginPlay`
  (`SceneComponent.SetVisibility` (`self.TextRender`) false false)
  (`SceneComponent.SetVisibility` (`self.TextRender1`) false false))

(event `what'sup`
  (`SceneComponent.SetVisibility` (`self.TextRender1`) true false)
  (`GameplayStatics.PlaySoundAtLocation` "/Game/StarterContent/Audio/_남성_흐흐흐흐_Cue._남성_흐흐흐흐_Cue" (0.0 0.0 0.0) (struct) 1.0 1.0 0.0 null null null))

(event `self.Box.OnComponentBeginOverlap`
  (params (OverlappedComponent :type "PrimitiveComponent Object Reference") (OtherActor :type "Actor Object Reference") (OtherComp :type "PrimitiveComponent Object Reference") (OtherBodyIndex :type Integer) (bFromSweep :type Boolean) (SweepResult :type "HitResult Structure (by ref)"))
  (if (== (`GameplayStatics.GetObjectClass` OtherActor) "/Game/BarrelHopper/Character/BH_Character.BH_Character_C")
    (if (`SceneComponent.IsVisible` (`self.TextRender1`))
      (`self.K2_DestroyActor`)
      (else
        (`SceneComponent.SetVisibility` (`self.TextRender`) true false)))))

(event `self.Box.OnComponentEndOverlap`
  (params (OverlappedComponent :type "PrimitiveComponent Object Reference") (OtherActor :type "Actor Object Reference") (OtherComp :type "PrimitiveComponent Object Reference") (OtherBodyIndex :type Integer))
  (if (== (`GameplayStatics.GetObjectClass` OtherActor) "/Game/BarrelHopper/Character/BH_Character.BH_Character_C")
    (`SceneComponent.SetVisibility` (`self.TextRender`) false false)))

(fn `Talk`
  (returns (Success :type Boolean))
  (`self.what'sup`)
  (return false))

(fn `UserConstructionScript`)